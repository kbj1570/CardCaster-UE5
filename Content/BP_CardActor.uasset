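; BP_CardActor is a card actor that initializes from the Crescent Lancer data asset and shows it through a widget component.
; Select raises the widget to a fixed height and Deselect returns it to the position stored at BeginPlay.
; Cursor-over plays the hover timeline only while selected, applying its Z offset on finish rather than per update.
; Cursor exit reverses that timeline only while unselected.
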(event Custom|Select
  (bind _originpos (Variables|Default|GetOriginPos))
  (Variables|Default|SetIsSelected true)
  (Transformation|SetRelativeLocation (Variables|Default|GetCardWidgetComp) (Math|Vector|MakeVector (.x _originpos) (.y _originpos) 4e+01) false false))

(event Custom|Deselect
  (Variables|Default|SetIsSelected false)
  (Transformation|SetRelativeLocation (Variables|Default|GetCardWidgetComp) (Variables|Default|GetOriginPos) false false))

(event EventBeginPlay
  (Class|CardActor|InitCard "/Game/CardData/DA_CrescentLancer.DA_CrescentLancer")
  (Variables|Default|SetOriginPos (Variables|/Script/Engine.SceneComponent|GetRelativeLocation (Variables|Default|GetCardWidgetComp))))

(event Collision|EventActorBeginOverlap
  (params (OtherActor :type Actor%20Object%20Reference)))

(event EventTick
  (params (DeltaSeconds :type Float%20%28single-precision%29)))

(event MouseInput|EventActorBeginCursorOver
  (if (Variables|Default|GetIsSelected)
    (bind _z_value (Timeline|HoverAnim Play)
      (:Finished
        (Transformation|SetRelativeLocation (Variables|Default|GetCardWidgetComp) (+ (Variables|Default|GetOriginPos) (.z (Math|Vector|MakeVector 0.0 0.0 _z_value))) false false)))))

(event MouseInput|EventActorEndCursorOver
  (if (not (Variables|Default|GetIsSelected))
    (bind _z_value (Timeline|HoverAnim Reverse)
      (:Finished
        (Transformation|SetRelativeLocation (Variables|Default|GetCardWidgetComp) (+ (Variables|Default|GetOriginPos) (.z (Math|Vector|MakeVector 0.0 0.0 _z_value))) false false)))))

(fn ConstructionScript)