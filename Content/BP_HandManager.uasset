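; Hand manager that spawns card actors into the player's hand and tracks which card is selected.
; SpawnCardInBP spawns a BP_CardActor at the manager's transform with a back-reference, initializes it from card data, adds it to CurrentHand and calls UpdateHandLayout.
; SelectCard acts only when a selection exists, deselecting that card, then clearing or replacing it.
; The construction script and NewFunction are empty.
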(event Custom|SelectCard
  (params (NewCard :type BP%20Card%20Actor%20Object%20Reference))
  (Utilities|IsValid (Variables|Default|GetSelectedCard)
    (:Is%20Valid
      (Default|Deselect (Variables|Default|GetSelectedCard))
      (if (== NewCard (Variables|Default|GetSelectedCard))
        (Variables|Default|SetSelectedCard 0)
        (else
          (Variables|Default|SetSelectedCard NewCard))))))

(event Custom|SpawnCardInBP
  (params (CardData :type Card%20Definition%20Object%20Reference))
  (bind _returnvalue (Game|SpawnActorfromClass "/Game/BP_CardActor.BP_CardActor_C" (Transformation|GetActorTransform) "Undefined" "MultiplyWithRoot" 0 self 0))
  (Class|CardActor|InitCard _returnvalue CardData)
  (Utilities|Array|Add (Variables|Default|GetCurrentHand) _returnvalue)
  (Class|HandManager|UpdateHandLayout))

(fn ConstructionScript)

(fn NewFunction)